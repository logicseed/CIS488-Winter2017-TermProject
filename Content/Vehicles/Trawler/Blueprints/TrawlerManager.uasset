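; Manager component on a Barge that keeps a school of nearby Trawlers moving in formation around it.
; At BeginPlay it finds Trawlers through the barge's detection component and requests each one's sequence position.
; Each tick it updates barge-relative positions and steers Trawlers there with AI MoveTo.
; A delay-driven timer periodically shifts the index offset, modulo four, intended to rotate the formation clockwise every ten seconds.
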(event EventBeginPlay
  ;[1 1 1] Getting owner components and moving trawlers to initial positions
  ;;[1 1 1] Get references to owners components
  (Utilities|FlowControl|Delay 0.1)
  (bind _returnvalue (CallFunction|GetTrawlerPositions))
  (Variables|Default|SettrawlerPositionComponent _returnvalue)
  (bind _returnvalue_2 (CallFunction|GetDetectOthers))
  (bind _output_get (Variables|Default|SetdetectOtherComponent _returnvalue_2))
  ;;[1 1 1] Find all trawlers within range and move them to your relative positions
  (bind _foundvehicles (Default|FindAllNearbyVehcileActorsOfType _output_get 5e+04 "/Game/Vehicles/Trawler/Trawler.Trawler_C"))
  (bind _output_get_2 (Variables|Default|Setschool _foundvehicles))
  (for (_array_element _array_index) _output_get_2
    (bind _astrawler (Utilities|Casting|CastToTrawler _array_element))
    (Default|GetSequencePosition _astrawler _array_index)
    (Variables|Default|SetInitialMoveDone true)))

(event EventTick
  (params (DeltaSeconds :type Float%20%28single-precision%29))
  ;[1 1 1] Trawler management logic
  (if (Variables|Default|GetInitialMoveDone)
    (Utilities|FlowControl|Sequence
      (:then_0
        ;;[1 1 1] Get updated positions after owner has moved
        (Default|UpdateRelativePositions (Variables|Default|GettrawlerPositionComponent)))
      (:then_1
        (if (== (Math|Integer|%(Integer) (stale _output_get) (stale _output_get_2)) 0)
          ;;[1 1 1] Create new movement configuration by rotating trawlers clockwise
          (bind _result (Math|Integer|IncrementInt (Variables|Default|GetcurrentPositionConfiguration))
            (:%20%20
              (Variables|Default|SetcurrentPositionConfiguration _result)
              (for (_array_element _array_index) (Variables|Default|Getschool)
                (bind _astrawler (Utilities|Casting|CastToTrawler _array_element))
                (bind _position (Default|GetSequencePosition _astrawler (Math|Integer|%(Integer) (+ _array_index (Variables|Default|GetcurrentPositionConfiguration)) 4)))
                (AI|AIMoveTo _astrawler _position 0 5.0 false))))
          (else
            ;;[1 1 1] Keep moving towards position
            (for (_array_element_2 _array_index_2) (Variables|Default|Getschool)
              (bind _astrawler_2 (Utilities|Casting|CastToTrawler _array_element_2))
              (bind _position_2 (Default|GetSequencePosition _astrawler_2 (Math|Integer|%(Integer) (+ _array_index_2 (Variables|Default|GetcurrentPositionConfiguration)) 4)))
              (AI|AIMoveTo _astrawler_2 _position_2 0 1e+01 false)))))
      (:then_2
        ;;[1 1 1] Track every 10 seconds
        (Utilities|FlowControl|Delay 1.0)
        (bind _result_2 (Math|Integer|IncrementInt (Variables|Default|Gettimer))
          (:%20%20
            (bind _output_get (Variables|Default|Settimer _result_2))
            (bind _output_get_2 (Variables|Default|SetdelayOnPositionChange 10))))))))

(fn GetTrawlerPositions
  (bind _asbarge (Utilities|Casting|CastToBarge (Components|GetOwner)))
  (bind _trawlerpositions (Default|GetTrawlerPosition _asbarge))
  (return _trawlerpositions))

(fn GetDetectOthers
  (bind _asbarge (Utilities|Casting|CastToBarge (Components|GetOwner)))
  (bind _detectothers (Default|GetDetectOthers _asbarge))
  (return _detectothers))