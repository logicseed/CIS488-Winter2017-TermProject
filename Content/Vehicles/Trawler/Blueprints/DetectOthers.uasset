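; Component in the Trawler vehicle's folder that detects other vehicle actors, such as the barge, near its owner.
; Each function runs a sphere overlap on the Vehicle object type at the owner's location, ignoring the owner.
; Queries return the first exact class match, all exact matches collected in FoundVehicles, or every overlapped actor.
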(fn FindSingleNearbyVehicleActor
  (params (SearchRadius :type Float%20%28single-precision%29) (VehicleActorToFind :type Actor%20Class%20Reference))
  ;[1 1 1] Check for the barge nearby
  (bind _outactors (Class|KismetSystemLibrary|SphereOverlapActorsNEW (Transformation|GetActorLocation (Components|GetOwner)) SearchRadius (Utilities|Array|MakeArray "ObjectTypeQuery5") 0 (Utilities|Array|MakeArray (Components|GetOwner))))
  (for _array_element _outactors
    (if (== (Utilities|GetClass _array_element) VehicleActorToFind)
      (return _array_element))))

(fn FindAllNearbyVehcileActorsOfType
  (params (SearchRadius :type Float%20%28single-precision%29) (VehicleActorToFind :type Actor%20Class%20Reference))
  (bind _foundvehicles (Variables|Default|GetFoundVehicles))
  (Utilities|Array|Clear (Variables|Default|GetFoundVehicles))
  (bind _outactors (Class|KismetSystemLibrary|SphereOverlapActorsNEW (Transformation|GetActorLocation (Components|GetOwner)) SearchRadius (Utilities|Array|MakeArray "ObjectTypeQuery5") 0 (Utilities|Array|MakeArray (Components|GetOwner))))
  (for _array_element _outactors
    (if (== (Utilities|GetClass _array_element) VehicleActorToFind)
      (Utilities|Array|Add _foundvehicles _array_element)))
  (return _foundvehicles))

(fn FindAllNearbyVehicleActors
  (params (SearchRadius :type Float%20%28single-precision%29))
  (Utilities|Array|Clear (Variables|Default|GetFoundVehicles))
  (bind _outactors (Class|KismetSystemLibrary|SphereOverlapActorsNEW (Transformation|GetActorLocation (Components|GetOwner)) SearchRadius (Utilities|Array|MakeArray "ObjectTypeQuery5") 0 (Utilities|Array|MakeArray (Components|GetOwner))))
  (return _outactors))