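; GroundControl handles ground driving for the player's Bashdozer vehicle, caching the player pawn on BeginPlay.
; MoveForward and MoveRight feed the vehicle movement, with engine idle and cruise audio switched on throttle and steering damped by half.
; SetHandbrake applies input only when the vehicle reports being on the ground.
; RightBashdozer flips it upright by teleporting the mesh with an offset, keeping yaw and optionally zeroing angular velocity.
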(event EventBeginPlay
  (bind _asbashdozer (Utilities|Casting|CastToBashdozer (Game|Player|GetPlayerPawn 0)))
  (Variables|Default|SetBashdozer _asbashdozer))

(event EventTick
  (params (DeltaSeconds :type Float%20%28single-precision%29)))

(fn RightBashdozer
  (params (WillResetAngularVelocity :type Boolean) (ChangeInLocation :type Vector))
  (bind _bashdozer (Variables|Default|GetBashdozer))
  (bind _mesh (Variables|/Script/Engine.WheeledVehicle|GetMesh _bashdozer))
  (if WillResetAngularVelocity
    (Class|PrimitiveComponent|SetPhysicsAngularVelocity _mesh "0, 0, 0" false "None"))
  (Transformation|SetWorldLocationAndRotation _mesh (+ ChangeInLocation (Transformation|GetWorldLocation _mesh)) (Math|Rotator|MakeRotator 0.0 0.0 (.Yaw (Math|Rotator|BreakRotator (Transformation|GetWorldRotation _mesh)))) false true))

(fn MoveForward
  (params (Throttle :type Float%20%28single-precision%29))
  (bind _bashdozer (Variables|Default|GetBashdozer))
  (bind _enginecruiseaudio (Variables|/Game/Vehicles/Bashdozer/Bashdozer.Bashdozer_C|GetEngineCruiseAudio _bashdozer))
  (Class|WheeledVehicleMovementComponent|SetThrottleInput (Variables|/Script/Engine.WheeledVehicle|GetVehicleMovement (Variables|Default|GetBashdozer)) Throttle)
  (if (Math|Float|NearlyEqual(Float) Throttle 0.0 0.0001)
    (Audio|Components|Audio|Stop (Variables|/Game/Vehicles/Bashdozer/Bashdozer.Bashdozer_C|GetEngineCruiseAudio (Variables|Default|GetBashdozer)))
    (if (not (Audio|Components|Audio|IsPlaying (Variables|/Game/Vehicles/Bashdozer/Bashdozer.Bashdozer_C|GetEngineIdleAudio (Variables|Default|GetBashdozer))))
      (Audio|Components|Audio|Play (Variables|/Game/Vehicles/Bashdozer/Bashdozer.Bashdozer_C|GetEngineIdleAudio (Variables|Default|GetBashdozer)) 0.0))
    (elif (not (Audio|Components|Audio|IsPlaying _enginecruiseaudio))
      (Audio|Components|Audio|Play _enginecruiseaudio 0.0)
      (Audio|Components|Audio|Stop (Variables|/Game/Vehicles/Bashdozer/Bashdozer.Bashdozer_C|GetEngineIdleAudio (Variables|Default|GetBashdozer))))))

(fn IsonGround
  (params (NewParam :type Boolean))
  (return (Variables|/Game/Vehicles/Bashdozer/Bashdozer.Bashdozer_C|GetOnGround (Variables|Default|GetBashdozer))))

(fn MoveRight
  (params (Steering :type Float%20%28single-precision%29))
  (Class|WheeledVehicleMovementComponent|SetSteeringInput (Variables|/Script/Engine.WheeledVehicle|GetVehicleMovement (Variables|Default|GetBashdozer)) (* Steering 0.5)))

(fn SetHandbrake
  (params (IsBraking :type Boolean))
  (bind _isonground (CallFunction|IsonGround false))
  (if _isonground
    (Class|WheeledVehicleMovementComponent|SetHandbrakeInput (Variables|/Script/Engine.WheeledVehicle|GetVehicleMovement (Variables|Default|GetBashdozer)) IsBraking)))