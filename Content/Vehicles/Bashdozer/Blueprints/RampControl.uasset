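; RampControl spawns Ramp actors in front of the player's Bashdozer vehicle.
; BeginPlay casts player pawn 0 to Bashdozer and caches the reference.
; SpawnRamp offsets the mesh location along its forward and up vectors by Distance and Height, plus an unscaled right vector, and matches the mesh rotation.
; Spawning adjusts for collisions where possible but always proceeds.
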(event EventBeginPlay
  (bind _asbashdozer (Utilities|Casting|CastToBashdozer (Game|Player|GetPlayerPawn 0))
    (:then
      _)
    (:CastFailed
      _))
  (Variables|Default|SetBashdozer _asbashdozer))

(event EventTick
  (params (DeltaSeconds :type Float%20%28single-precision%29)))

(fn SpawnRamp
  (bind _bashdozer (Variables|Default|GetBashdozer))
  (bind _mesh (Variables|/Script/Engine.WheeledVehicle|GetMesh _bashdozer))
  (Game|SpawnActorfromClass "/Game/Gameplay/Ramp/Ramp.Ramp_C" (Math|Transform|MakeTransform (+ (* (Math|Vector|GetForwardVector _mesh) (Variables|Default|GetDistance)) (* (Math|Vector|GetUpVector _mesh) (Variables|Default|GetHeight)) (Math|Vector|GetRightVector _mesh) (Transformation|GetWorldLocation _mesh)) (Transformation|GetWorldRotation _mesh)) "AdjustIfPossibleButAlwaysSpawn" 0 0))