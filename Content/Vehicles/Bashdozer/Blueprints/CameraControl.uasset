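; Camera helper for the Bashdozer vehicle that rotates the player pawn's boom for look input.
; BeginPlay caches player pawn 0 as a Bashdozer, and the look and reset functions act on that pawn's Boom.
; LookUp and LookRight add sensitivity-scaled input to relative pitch and yaw without clamping, with LookRight also zeroing roll.
; ResetCamera snaps the boom to the mesh's world rotation; references stored by Initialize go unused here.
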(event EventTick
  (params (DeltaSeconds :type Float%20%28single-precision%29)))

(event EventBeginPlay
  (bind _asbashdozer (Utilities|Casting|CastToBashdozer (Game|Player|GetPlayerPawn 0))
    (:then
      _)
    (:CastFailed
      _))
  (Variables|Default|SetBashdozer _asbashdozer))

(fn Initialize
  (params (Boom :type Spring%20Arm%20Component%20Object%20Reference) (Mesh :type Skeletal%20Mesh%20Component%20Object%20Reference))
  (Variables|Default|SetBoom Boom)
  (Variables|Default|SetMesh Mesh))

(fn ResetCamera
  (Transformation|SetWorldRotation (Variables|/Game/Vehicles/Bashdozer/Bashdozer.Bashdozer_C|GetBoom (Variables|Default|GetBashdozer)) (Transformation|GetWorldRotation (Variables|/Script/Engine.WheeledVehicle|GetMesh (Variables|Default|GetBashdozer))) false true))

(fn LookUp
  (params (AxisValue :type Float%20%28single-precision%29))
  (bind _bashdozer (Variables|Default|GetBashdozer))
  (bind _boom (Variables|/Game/Vehicles/Bashdozer/Bashdozer.Bashdozer_C|GetBoom _bashdozer))
  (bind _relativerotation (Variables|/Script/Engine.SceneComponent|GetRelativeRotation _boom))
  (bind (_roll _pitch _yaw) (Math|Rotator|BreakRotator _relativerotation))
  (Transformation|SetRelativeRotation (Variables|/Game/Vehicles/Bashdozer/Bashdozer.Bashdozer_C|GetBoom (Variables|Default|GetBashdozer)) (Math|Rotator|MakeRotator _roll (+ (* AxisValue (Variables|Default|GetCamera%20Senstivity)) _pitch) _yaw) false false))

(fn LookRight
  (params (AxisValue :type Float%20%28single-precision%29))
  (bind _bashdozer (Variables|Default|GetBashdozer))
  (bind _boom (Variables|/Game/Vehicles/Bashdozer/Bashdozer.Bashdozer_C|GetBoom _bashdozer))
  (bind _relativerotation (Variables|/Script/Engine.SceneComponent|GetRelativeRotation _boom))
  (bind (_roll _pitch _yaw) (Math|Rotator|BreakRotator _relativerotation))
  (Transformation|SetRelativeRotation (Variables|/Game/Vehicles/Bashdozer/Bashdozer.Bashdozer_C|GetBoom (Variables|Default|GetBashdozer)) (Math|Rotator|MakeRotator 0.0 _pitch (+ (* AxisValue (Variables|Default|GetCamera%20Senstivity)) _yaw)) false false))