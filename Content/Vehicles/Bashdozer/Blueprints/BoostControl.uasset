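; BoostControl manages a limited boost meter for the player's Bashdozer, which it finds from the player pawn on BeginPlay.
; BoostForward spends a fixed amount per call, pushes the mesh along its forward axis as a scaled acceleration, and restarts the recharge delay.
; Tick refills the meter at a constant, frame-rate-independent rate once that delay passes, while boost drain is per call.
; An unconnected IsBoosting loop never runs.
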(event EventBeginPlay
  (bind _asbashdozer (Utilities|Casting|CastToBashdozer (Game|Player|GetPlayerPawn 0)))
  (Variables|Default|SetBashdozer _asbashdozer)
  (Variables|Default|SetCurrentBoost (Variables|Default|GetMaxBoost)))

(event EventTick
  (params (DeltaSeconds :type Float%20%28single-precision%29))
  (if (and (< (Variables|Default|GetChargeCooldownTime) (Utilities|Time|GetGameTimeinSeconds)) (> (Variables|Default|GetMaxBoost) (Variables|Default|GetCurrentBoost)))
    (Variables|Default|SetCurrentBoost (+ (Variables|Default|GetCurrentBoost) (* DeltaSeconds 1e+01)))))

(fn BoostForward
  (params (Boost :type Float%20%28single-precision%29))
  (bind _bashdozer (Variables|Default|GetBashdozer))
  (bind _mesh (Variables|/Script/Engine.WheeledVehicle|GetMesh _bashdozer))
  (if (> Boost 0.0)
    (if (>= (Variables|Default|GetCurrentBoost) 0.0)
      (Variables|Default|SetChargeCooldownTime (+ (Utilities|Time|GetGameTimeinSeconds) (Variables|Default|GetBoostChargeDelay)))
      (Variables|Default|SetCurrentBoost (- (Variables|Default|GetCurrentBoost) 1.0))
      (Physics|AddForce _mesh (* (* (Math|Vector|RotateVector "1.000000, 0, 0" (Transformation|GetWorldRotation _mesh)) Boost) 3e+03) "None" true))))