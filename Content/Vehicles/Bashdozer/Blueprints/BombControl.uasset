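; Bomb controller for the player's Bashdozer vehicle, providing aft, port, starboard and paired belly bombs that boost it in mesh-relative directions.
; Detonation starts a cooldown, zeroes vertical velocity plus pitch and roll spin, applies a mass-independent force with effects, and destroys the bomb actor.
; Tick checks each cooldown against game time, then respawns the color-coded bomb actors attached to their vehicle sockets.
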(event EventBeginPlay
  (bind _asbashdozer (Utilities|Casting|CastToBashdozer (Game|Player|GetPlayerPawn 0)))
  (Variables|Default|SetBashdozer _asbashdozer)
  (Graphics|SpawnAllBombs))

(event EventTick
  (params (DeltaSeconds :type Float%20%28single-precision%29))
  (Cooldown|UpdateAllCooldowns))

(fn AftBomb
  (if (Variables|Cooldown|GetAftBombIsReady)
    (Cooldown|StartCooldown (Variables|Cooldown|GetAftCooldownTime) (Variables|Cooldown|GetAftBombIsReady))
    ;[1 1 1] Comment
    (bind _returnvalue (Physics|GetPhysicsLinearVelocity (Variables|/Script/Engine.WheeledVehicle|GetMesh (Variables|Default|GetBashdozer)) "None"))
    (Physics|SetPhysicsLinearVelocity (Variables|/Script/Engine.WheeledVehicle|GetMesh (Variables|Default|GetBashdozer)) (Math|Vector|MakeVector (.X (Math|Vector|BreakVector _returnvalue)) (.Y (Math|Vector|BreakVector _returnvalue)) 0.0) false "None")
    (bind _returnvalue_2 (Class|PrimitiveComponent|GetPhysicsAngularVelocity (Variables|/Script/Engine.WheeledVehicle|GetMesh (Variables|Default|GetBashdozer)) "None"))
    (Class|PrimitiveComponent|SetPhysicsAngularVelocity (Variables|/Script/Engine.WheeledVehicle|GetMesh (Variables|Default|GetBashdozer)) (Math|Vector|MakeVector 0.0 0.0 (.Z (Math|Vector|BreakVector _returnvalue_2))) false "None")
    (Detonation|DetonateBomb "0,0.000000,-1.000000" (Variables|Detonation|GetAftBombStrength) (Variables|/Game/Vehicles/Bashdozer/Bashdozer.Bashdozer_C|GetAftBombEffect (Variables|Default|GetBashdozer)))
    (Actor|DestroyActor (Variables|Graphics|GetAftBombGraphic))))

(fn BellyBombs
  (if (Variables|Cooldown|GetBellyBombsAreReady)
    (Cooldown|StartCooldown (Variables|Cooldown|GetBellyCooldownTime) (Variables|Cooldown|GetBellyBombsAreReady))
    ;[1 1 1] Comment
    (bind _returnvalue (Physics|GetPhysicsLinearVelocity (Variables|/Script/Engine.WheeledVehicle|GetMesh (Variables|Default|GetBashdozer)) "None"))
    (Physics|SetPhysicsLinearVelocity (Variables|/Script/Engine.WheeledVehicle|GetMesh (Variables|Default|GetBashdozer)) (Math|Vector|MakeVector (.X (Math|Vector|BreakVector _returnvalue)) (.Y (Math|Vector|BreakVector _returnvalue)) 0.0) false "None")
    (bind _returnvalue_2 (Class|PrimitiveComponent|GetPhysicsAngularVelocity (Variables|/Script/Engine.WheeledVehicle|GetMesh (Variables|Default|GetBashdozer)) "None"))
    (Class|PrimitiveComponent|SetPhysicsAngularVelocity (Variables|/Script/Engine.WheeledVehicle|GetMesh (Variables|Default|GetBashdozer)) (Math|Vector|MakeVector 0.0 0.0 (.Z (Math|Vector|BreakVector _returnvalue_2))) false "None")
    (Detonation|DetonateBomb "0,0.000000,1.000000" (Variables|Detonation|GetBellyBombStrength) (Variables|/Game/Vehicles/Bashdozer/Bashdozer.Bashdozer_C|GetBellyBombEffectF (Variables|Default|GetBashdozer)))
    (Components|Activation|Activate (Variables|/Game/Vehicles/Bashdozer/Bashdozer.Bashdozer_C|GetBellyBombEffectR (Variables|Default|GetBashdozer)) true)
    (Actor|DestroyActor (Variables|Graphics|GetBellyBombFGraphic))
    (Actor|DestroyActor (Variables|Graphics|GetBellyBombRGraphic))))

(fn PortBomb
  (if (Variables|Cooldown|GetPortBombIsReady)
    (Cooldown|StartCooldown (Variables|Cooldown|GetPortCooldownTime) (Variables|Cooldown|GetPortBombIsReady))
    ;[1 1 1] Comment
    (bind _returnvalue (Physics|GetPhysicsLinearVelocity (Variables|/Script/Engine.WheeledVehicle|GetMesh (Variables|Default|GetBashdozer)) "None"))
    (Physics|SetPhysicsLinearVelocity (Variables|/Script/Engine.WheeledVehicle|GetMesh (Variables|Default|GetBashdozer)) (Math|Vector|MakeVector (.X (Math|Vector|BreakVector _returnvalue)) (.Y (Math|Vector|BreakVector _returnvalue)) 0.0) false "None")
    (bind _returnvalue_2 (Class|PrimitiveComponent|GetPhysicsAngularVelocity (Variables|/Script/Engine.WheeledVehicle|GetMesh (Variables|Default|GetBashdozer)) "None"))
    (Class|PrimitiveComponent|SetPhysicsAngularVelocity (Variables|/Script/Engine.WheeledVehicle|GetMesh (Variables|Default|GetBashdozer)) (Math|Vector|MakeVector 0.0 0.0 (.Z (Math|Vector|BreakVector _returnvalue_2))) false "None")
    (Detonation|DetonateBomb "0,1.000000,0.000000" (Variables|Detonation|GetPortBombStrength) (Variables|/Game/Vehicles/Bashdozer/Bashdozer.Bashdozer_C|GetPortBombEffect (Variables|Default|GetBashdozer)))
    (Actor|DestroyActor (Variables|Graphics|GetPortBombGraphic))))

(fn StarboardBomb
  (if (Variables|Cooldown|GetStarboardBombIsReady)
    (Cooldown|StartCooldown (Variables|Cooldown|GetStarboardCooldownTime) (Variables|Cooldown|GetStarboardBombIsReady))
    ;[1 1 1] Comment
    (bind _returnvalue (Physics|GetPhysicsLinearVelocity (Variables|/Script/Engine.WheeledVehicle|GetMesh (Variables|Default|GetBashdozer)) "None"))
    (Physics|SetPhysicsLinearVelocity (Variables|/Script/Engine.WheeledVehicle|GetMesh (Variables|Default|GetBashdozer)) (Math|Vector|MakeVector (.X (Math|Vector|BreakVector _returnvalue)) (.Y (Math|Vector|BreakVector _returnvalue)) 0.0) false "None")
    (bind _returnvalue_2 (Class|PrimitiveComponent|GetPhysicsAngularVelocity (Variables|/Script/Engine.WheeledVehicle|GetMesh (Variables|Default|GetBashdozer)) "None"))
    (Class|PrimitiveComponent|SetPhysicsAngularVelocity (Variables|/Script/Engine.WheeledVehicle|GetMesh (Variables|Default|GetBashdozer)) (Math|Vector|MakeVector 0.0 0.0 (.Z (Math|Vector|BreakVector _returnvalue_2))) false "None")
    (Detonation|DetonateBomb "0,-1.000000,0.000000" (Variables|Detonation|GetStarboardBombStrength) (Variables|/Game/Vehicles/Bashdozer/Bashdozer.Bashdozer_C|GetStarboardBombEffect (Variables|Default|GetBashdozer)))
    (Actor|DestroyActor (Variables|Graphics|GetStarboardBombGraphic))))

(fn DetonateBomb
  (params (Direction :type Vector) (Magnitude :type Float%20%28single-precision%29) (Effect :type Particle%20System%20Component%20Object%20Reference%20%28by%20ref%29))
  (Components|Activation|Activate Effect true)
  (Physics|AddForce (Variables|/Script/Engine.WheeledVehicle|GetMesh (Variables|Default|GetBashdozer)) (* (* (Math|Vector|RotateVector Direction (Transformation|GetWorldRotation (Variables|/Script/Engine.WheeledVehicle|GetMesh (Variables|Default|GetBashdozer)))) Magnitude) (Variables|Detonation|GetBombCorrectionFactor)) "None" true))

(fn UpdateCooldown
  (params (Ready :type Boolean%20%28by%20ref%29) (CooldownTimer :type Float%20%28single-precision%29%20%28by%20ref%29) (BombSocket :type BombSockets%20Enum))
  (if (not Ready)
    (if (< CooldownTimer (Utilities|Time|GetGameTimeinSeconds))
      (|SetBy-RefVar Ready true)
      (switch Utilities|FlowControl|Switch|SwitchonBombSockets BombSocket
        (:NewEnumerator0
          (Graphics|SpawnAftBomb))
        (:NewEnumerator1
          (Graphics|SpawnBellyBombF)
          (Graphics|SpawnBellyBombR))
        (:NewEnumerator2
          (Graphics|SpawnPortBomb))
        (:NewEnumerator3
          (Graphics|SpawnStarboardBomb))))))

(fn SpawnBombGraphic
  (params (Socket%20Name :type Name) (BombGraphic :type Bomb%20Object%20Reference%20%28by%20ref%29))
  (bind _returnvalue (Game|SpawnActorfromClass "/Game/Gameplay/Bombs/Bomb.Bomb_C" (Transformation|GetSocketTransform (Variables|/Script/Engine.WheeledVehicle|GetMesh (Variables|Default|GetBashdozer)) Socket%20Name "RTS_Actor") "Undefined" 0 0))
  (|SetBy-RefVar BombGraphic _returnvalue)
  (Transformation|AttachActorToActor BombGraphic (Variables|Default|GetBashdozer) Socket%20Name "SnapToTarget" "SnapToTarget" "KeepRelative" true)
  (return))

(fn SpawnAllBombs
  (Utilities|FlowControl|Sequence
    (:then_0
      (Graphics|SpawnAftBomb))
    (:then_1
      (Graphics|SpawnBellyBombF))
    (:then_2
      (Graphics|SpawnBellyBombR))
    (:then_3
      (Graphics|SpawnPortBomb))
    (:then_4
      (Graphics|SpawnStarboardBomb))))

(fn DetroyBomb
  (Actor|DestroyActor (Variables|Graphics|GetAftBombGraphic)))

(fn StartCooldown
  (params (CooldownTimer :type Float%20%28single-precision%29%20%28by%20ref%29) (ReadyCheck :type Boolean%20%28by%20ref%29))
  (|SetBy-RefVar ReadyCheck false)
  (|SetBy-RefVar CooldownTimer (+ (Utilities|Time|GetGameTimeinSeconds) (Variables|Cooldown|GetCooldownLength))))

(fn UpdateAllCooldowns
  (Cooldown|UpdateCooldown (Variables|Cooldown|GetAftBombIsReady) (Variables|Cooldown|GetAftCooldownTime) "NewEnumerator0")
  (Cooldown|UpdateCooldown (Variables|Cooldown|GetBellyBombsAreReady) (Variables|Cooldown|GetBellyCooldownTime) "NewEnumerator1")
  (Cooldown|UpdateCooldown (Variables|Cooldown|GetPortBombIsReady) (Variables|Cooldown|GetPortCooldownTime) "NewEnumerator2")
  (Cooldown|UpdateCooldown (Variables|Cooldown|GetStarboardBombIsReady) (Variables|Cooldown|GetStarboardCooldownTime) "NewEnumerator3"))

(fn SpawnAftBomb
  (Graphics|SpawnBombGraphic "AftBombSocket" (Variables|Graphics|GetAftBombGraphic))
  (Rendering|Material|SetMaterialbyName (Variables|/Game/Gameplay/Bombs/Bomb.Bomb_C|GetStaticMesh (Variables|Graphics|GetAftBombGraphic)) "Bomb_Material" "/Game/Gameplay/Bombs/Bomb_Material_Yellow.Bomb_Material_Yellow"))

(fn SpawnBellyBombF
  (Graphics|SpawnBombGraphic "BellyBombFSocket" (Variables|Graphics|GetBellyBombFGraphic))
  (Rendering|Material|SetMaterialbyName (Variables|/Game/Gameplay/Bombs/Bomb.Bomb_C|GetStaticMesh (Variables|Graphics|GetBellyBombFGraphic)) "Bomb_Material" "/Game/Gameplay/Bombs/Bomb_Material_Green.Bomb_Material_Green"))

(fn SpawnBellyBombR
  (Graphics|SpawnBombGraphic "BellyBombRSocket" (Variables|Graphics|GetBellyBombRGraphic))
  (Rendering|Material|SetMaterialbyName (Variables|/Game/Gameplay/Bombs/Bomb.Bomb_C|GetStaticMesh (Variables|Graphics|GetBellyBombRGraphic)) "Bomb_Material" "/Game/Gameplay/Bombs/Bomb_Material_Green.Bomb_Material_Green"))

(fn SpawnPortBomb
  (Graphics|SpawnBombGraphic "PortBombSocket" (Variables|Graphics|GetPortBombGraphic))
  (Rendering|Material|SetMaterialbyName (Variables|/Game/Gameplay/Bombs/Bomb.Bomb_C|GetStaticMesh (Variables|Graphics|GetPortBombGraphic)) "Bomb_Material" "/Game/Gameplay/Bombs/Bomb_Material_Blue.Bomb_Material_Blue"))

(fn SpawnStarboardBomb
  (Graphics|SpawnBombGraphic "StarboardBombSocket" (Variables|Graphics|GetStarboardBombGraphic))
  (Rendering|Material|SetMaterialbyName (Variables|/Game/Gameplay/Bombs/Bomb.Bomb_C|GetStaticMesh (Variables|Graphics|GetStarboardBombGraphic)) "Bomb_Material" "/Game/Gameplay/Bombs/Bomb_Material_Red.Bomb_Material_Red"))