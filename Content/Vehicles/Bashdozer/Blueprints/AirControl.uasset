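; Air control Blueprint for the Bashdozer vehicle that rolls and pitches its mesh from axis input.
; BeginPlay casts player pawn 0 to Bashdozer and caches the reference.
; RollRight and PitchUp add scaled input to the mesh's world roll or pitch, applied as a teleport at the current location.
; Rotation steps are per call, with no delta-time scaling or airborne check here.
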(event EventBeginPlay
  (bind _asbashdozer (Utilities|Casting|CastToBashdozer (Game|Player|GetPlayerPawn 0)))
  (Variables|Default|SetBashdozer _asbashdozer))

(event EventTick
  (params (DeltaSeconds :type Float%20%28single-precision%29)))

(fn RollRight
  (params (InputAxis :type Float%20%28single-precision%29))
  (bind _bashdozer (Variables|Default|GetBashdozer))
  (bind _mesh (Variables|/Script/Engine.WheeledVehicle|GetMesh _bashdozer))
  (bind _returnvalue (Transformation|GetWorldRotation _mesh))
  (bind (_roll _pitch _yaw) (Math|Rotator|BreakRotator _returnvalue))
  (Transformation|SetWorldLocationAndRotation (Variables|/Script/Engine.WheeledVehicle|GetMesh (Variables|Default|GetBashdozer)) (Transformation|GetWorldLocation (Variables|/Script/Engine.WheeledVehicle|GetMesh (Variables|Default|GetBashdozer))) (Math|Rotator|MakeRotator (+ (* InputAxis 3.0) _roll) _pitch _yaw) false true))

(fn PitchUp
  (params (InputAxis :type Float%20%28single-precision%29))
  (bind _bashdozer (Variables|Default|GetBashdozer))
  (bind _mesh (Variables|/Script/Engine.WheeledVehicle|GetMesh _bashdozer))
  (bind _returnvalue (Transformation|GetWorldRotation _mesh))
  (bind (_roll _pitch _yaw) (Math|Rotator|BreakRotator _returnvalue))
  (Transformation|SetWorldLocationAndRotation _mesh (Transformation|GetWorldLocation _mesh) (Math|Rotator|MakeRotator _roll (+ (* InputAxis (LocalVariables|Getconst)) _pitch) _yaw) false true))