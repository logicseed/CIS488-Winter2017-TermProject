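; Component that computes a ring of slot positions around its owner, one per trawler, on a world-aligned ellipse with semi-axes A and B.
; UpdateRelativePositions steps evenly by angle, traces down against WorldStatic for height and stores relative offsets in Debug.
; Theta advances between trace and store, so each slot's height comes from the previous angle's trace.
; GetPosition returns a stored slot by index.
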(fn UpdateRelativePositions
  (params (NumberOfTrawlers :type Array%20of%20Actor%20Object%20References))
  (bind _returnvalue (Components|GetOwner))
  (bind _a (Variables|Default|GetA))
  (bind _b (Variables|Default|GetB))
  (bind _returnvalue_2 (Math|Float|Square _b))
  (bind _returnvalue_3 (Math|Float|Square _a))
  (bind _returnvalue_4 (Transformation|GetActorLocation _returnvalue))
  (bind _returnvalue_5 (* _a _b))
  (bind (_x _y _z) (Math|Vector|BreakVector _returnvalue_4))
  ;[1 1 1] Update positions relative to the owners positions
  (Utilities|Array|Clear (Variables|Default|Getdebug))
  (Utilities|Array|Clear (Variables|Default|GetpossiblePositions))
  (Variables|Default|SetDeltaTheta (/ 3.6e+02 (Math|Conversions|ToFloat(Integer) (Utilities|Array|Length NumberOfTrawlers))))
  (for _array_element NumberOfTrawlers
    (bind _outhit (Collision|LineTraceForObjects (Math|Vector|MakeVector (+ _x (Math|Float|SelectFloat (* -1.0 (/ _returnvalue_5 (Math|Float|Sqrt (+ (* (Math|Float|Square (Math|Trig|Tan(Degrees) (Variables|Default|GetTheta))) _returnvalue_3) _returnvalue_2)))) (/ _returnvalue_5 (Math|Float|Sqrt (+ (* (Math|Float|Square (Math|Trig|Tan(Degrees) (Variables|Default|GetTheta))) _returnvalue_3) _returnvalue_2))) (Math|Float|InRange(Float) (Variables|Default|GetTheta) 9e+01 2.7e+02))) (+ _y (Math|Float|SelectFloat (/ _returnvalue_5 (Math|Float|Sqrt (+ _returnvalue_3 (/ _returnvalue_2 (Math|Float|Square (Math|Trig|Tan(Degrees) (Variables|Default|GetTheta))))))) (* -1.0 (/ _returnvalue_5 (Math|Float|Sqrt (+ _returnvalue_3 (/ _returnvalue_2 (Math|Float|Square (Math|Trig|Tan(Degrees) (Variables|Default|GetTheta)))))))) (Math|Float|InRange(Float) (Variables|Default|GetTheta) 0.0 1.8e+02))) _z) (- (Math|Vector|MakeVector (+ _x (Math|Float|SelectFloat (* -1.0 (/ _returnvalue_5 (Math|Float|Sqrt (+ (* (Math|Float|Square (Math|Trig|Tan(Degrees) (Variables|Default|GetTheta))) _returnvalue_3) _returnvalue_2)))) (/ _returnvalue_5 (Math|Float|Sqrt (+ (* (Math|Float|Square (Math|Trig|Tan(Degrees) (Variables|Default|GetTheta))) _returnvalue_3) _returnvalue_2))) (Math|Float|InRange(Float) (Variables|Default|GetTheta) 9e+01 2.7e+02))) (+ _y (Math|Float|SelectFloat (/ _returnvalue_5 (Math|Float|Sqrt (+ _returnvalue_3 (/ _returnvalue_2 (Math|Float|Square (Math|Trig|Tan(Degrees) (Variables|Default|GetTheta))))))) (* -1.0 (/ _returnvalue_5 (Math|Float|Sqrt (+ _returnvalue_3 (/ _returnvalue_2 (Math|Float|Square (Math|Trig|Tan(Degrees) (Variables|Default|GetTheta)))))))) (Math|Float|InRange(Float) (Variables|Default|GetTheta) 0.0 1.8e+02))) _z) (* "0, 0,1.000000" (Variables|Default|GettraceRange))) (Utilities|Array|MakeArray "ObjectTypeQuery1") false 0 "None" true "(R=1.000000,G=0.000000,B=0.000000,A=1.000000)" "(R=0.000000,G=1.000000,B=0.000000,A=1.000000)" 2.0))
    (Variables|Default|SetTheta (+ (Variables|Default|GetDeltaTheta) (Variables|Default|GetTheta)))
    (Utilities|Array|Add (Variables|Default|GetpossiblePositions) (Math|Vector|MakeVector (.X (Math|Vector|BreakVector (Math|Vector|MakeVector (+ _x (Math|Float|SelectFloat (* -1.0 (/ _returnvalue_5 (Math|Float|Sqrt (+ (* (Math|Float|Square (Math|Trig|Tan(Degrees) (Variables|Default|GetTheta))) _returnvalue_3) _returnvalue_2)))) (/ _returnvalue_5 (Math|Float|Sqrt (+ (* (Math|Float|Square (Math|Trig|Tan(Degrees) (Variables|Default|GetTheta))) _returnvalue_3) _returnvalue_2))) (Math|Float|InRange(Float) (Variables|Default|GetTheta) 9e+01 2.7e+02))) (+ _y (Math|Float|SelectFloat (/ _returnvalue_5 (Math|Float|Sqrt (+ _returnvalue_3 (/ _returnvalue_2 (Math|Float|Square (Math|Trig|Tan(Degrees) (Variables|Default|GetTheta))))))) (* -1.0 (/ _returnvalue_5 (Math|Float|Sqrt (+ _returnvalue_3 (/ _returnvalue_2 (Math|Float|Square (Math|Trig|Tan(Degrees) (Variables|Default|GetTheta)))))))) (Math|Float|InRange(Float) (Variables|Default|GetTheta) 0.0 1.8e+02))) _z))) (.Y (Math|Vector|BreakVector (Math|Vector|MakeVector (+ _x (Math|Float|SelectFloat (* -1.0 (/ _returnvalue_5 (Math|Float|Sqrt (+ (* (Math|Float|Square (Math|Trig|Tan(Degrees) (Variables|Default|GetTheta))) _returnvalue_3) _returnvalue_2)))) (/ _returnvalue_5 (Math|Float|Sqrt (+ (* (Math|Float|Square (Math|Trig|Tan(Degrees) (Variables|Default|GetTheta))) _returnvalue_3) _returnvalue_2))) (Math|Float|InRange(Float) (Variables|Default|GetTheta) 9e+01 2.7e+02))) (+ _y (Math|Float|SelectFloat (/ _returnvalue_5 (Math|Float|Sqrt (+ _returnvalue_3 (/ _returnvalue_2 (Math|Float|Square (Math|Trig|Tan(Degrees) (Variables|Default|GetTheta))))))) (* -1.0 (/ _returnvalue_5 (Math|Float|Sqrt (+ _returnvalue_3 (/ _returnvalue_2 (Math|Float|Square (Math|Trig|Tan(Degrees) (Variables|Default|GetTheta)))))))) (Math|Float|InRange(Float) (Variables|Default|GetTheta) 0.0 1.8e+02))) _z))) (.Z (Math|Vector|BreakVector (.Location (Collision|BreakHitResult _outhit))))))
    (Utilities|Array|Add (Variables|Default|Getdebug) (Math|Vector|MakeVector (Math|Float|SelectFloat (* -1.0 (/ _returnvalue_5 (Math|Float|Sqrt (+ (* (Math|Float|Square (Math|Trig|Tan(Degrees) (Variables|Default|GetTheta))) _returnvalue_3) _returnvalue_2)))) (/ _returnvalue_5 (Math|Float|Sqrt (+ (* (Math|Float|Square (Math|Trig|Tan(Degrees) (Variables|Default|GetTheta))) _returnvalue_3) _returnvalue_2))) (Math|Float|InRange(Float) (Variables|Default|GetTheta) 9e+01 2.7e+02)) (Math|Float|SelectFloat (/ _returnvalue_5 (Math|Float|Sqrt (+ _returnvalue_3 (/ _returnvalue_2 (Math|Float|Square (Math|Trig|Tan(Degrees) (Variables|Default|GetTheta))))))) (* -1.0 (/ _returnvalue_5 (Math|Float|Sqrt (+ _returnvalue_3 (/ _returnvalue_2 (Math|Float|Square (Math|Trig|Tan(Degrees) (Variables|Default|GetTheta)))))))) (Math|Float|InRange(Float) (Variables|Default|GetTheta) 0.0 1.8e+02)) 0.0)))
  (Variables|Default|SetTheta 0.0)
  (return))

(fn GetPosition
  (params (positionIndex :type Integer))
  (return (Utilities|Array|Get(acopy) (Variables|Default|GetpossiblePositions) positionIndex)))