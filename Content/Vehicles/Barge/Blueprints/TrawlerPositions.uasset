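; Barge component that provides positions around the barge, apparently for its trawlers.
; UpdateRelativePositions rebuilds four corner points from the barge's location plus or minus X and Y offset vectors, ignoring its NumberOfTrawlers input.
; A downward trace against WorldStatic sets each point's height, without checking for a hit.
; GetPosition returns a stored point by index.
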(fn UpdateRelativePositions
  (params (NumberOfTrawlers :type Array%20of%20Actor%20Object%20References))
  (bind _xpositionoffset (Variables|Default|GetxPositionOffset))
  (bind _ypositionoffset (Variables|Default|GetyPositionOffset))
  (bind _returnvalue (Math|Vector|NegateVector _xpositionoffset))
  (bind _returnvalue_2 (Math|Vector|NegateVector _ypositionoffset))
  ;[1 1 1] Update positions relative to the owners positions
  (bind _asbarge (Utilities|Casting|CastToBarge (Components|GetOwner)))
  (Utilities|Array|Clear (Variables|Default|GetpossiblePositions))
  (for _array_element (Utilities|Array|MakeArray (+ (Transformation|GetActorLocation _asbarge) (+ _xpositionoffset _ypositionoffset)) (+ (Transformation|GetActorLocation _asbarge) (+ _xpositionoffset _returnvalue_2)) (+ (Transformation|GetActorLocation _asbarge) (+ _returnvalue _returnvalue_2)) (+ (Transformation|GetActorLocation _asbarge) (+ _returnvalue _ypositionoffset)))
    (bind _outhit (Collision|LineTraceForObjects _array_element (- _array_element (* "0, 0,1.000000" (Variables|Default|GettraceRange))) (Utilities|Array|MakeArray "ObjectTypeQuery1") false 0 "None" true "(R=1.000000,G=0.000000,B=0.000000,A=1.000000)" "(R=0.000000,G=1.000000,B=0.000000,A=1.000000)" 2.0))
    (Utilities|Array|Add (Variables|Default|GetpossiblePositions) (Math|Vector|MakeVector (.X (Math|Vector|BreakVector _array_element)) (.Y (Math|Vector|BreakVector _array_element)) (.Z (Math|Vector|BreakVector (.Location (Collision|BreakHitResult _outhit)))))))
  (return))

(fn GetPosition
  (params (positionIndex :type Integer))
  (return (Utilities|Array|Get(acopy) (Variables|Default|GetpossiblePositions) positionIndex)))