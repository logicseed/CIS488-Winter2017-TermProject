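; Barge component that manages nearby trawlers, keeping them in formation slots around the barge and periodically rotating them.
; On BeginPlay, after a short delay, it caches the barge's position and detection components and gathers trawlers in range into School.
; Each tick updates relative positions and sends each trawler to its slot, offset by a shared configuration index.
; A Delay-driven seconds counter advances that index at intervals, with modulo wrapping the slots.
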(event EventBeginPlay
  ;[1 1 1] Getting owner components and moving trawlers to initial positions
  ;;[1 1 1] Get references to owners components
  (Utilities|FlowControl|Delay 0.1)
  (bind _trawlerpositionsv2 (CallFunction|GetTrawlerPositions))
  (Variables|Default|SetPositionComponent _trawlerpositionsv2)
  (bind _returnvalue (CallFunction|GetDetectOthers))
  (bind _output_get (Variables|Default|SetdetectOtherComponent _returnvalue))
  ;;[1 1 1] Find all trawlers within range
  (bind _foundvehicles (Default|FindAllNearbyVehcileActorsOfType _output_get 5e+03 "/Game/Vehicles/Trawler/Trawler.Trawler_C"))
  (for _array_element _foundvehicles
    (Utilities|Array|Add (Variables|Default|Getschool) _array_element))
  (Variables|Default|SetsetUpDone true))

(event EventTick
  (params (DeltaSeconds :type Float%20%28single-precision%29))
  (bind _school (Variables|Default|Getschool))
  ;[1 1 1] Trawler management logic
  (if (Variables|Default|GetsetUpDone)
    (Utilities|FlowControl|Sequence
      (:then_0
        ;;[1 1 1] Get updated positions after owner has moved
        (Default|UpdateRelativePositions (Variables|Default|GetPositionComponent) _school))
      (:then_1
        (if (== (Math|Integer|%(Integer) (stale _output_get) (+ (Variables|Default|GetdelayOnPositionChange) 1)) 0)
          ;;[1 1 1] Create new movement configuration by rotating trawlers clockwise
          (bind _result (Math|Integer|IncrementInt (Variables|Default|GetcurrentPositionConfiguration))
            (:%20%20
              (Variables|Default|SetcurrentPositionConfiguration _result)
              (bind _result_2 (Math|Integer|IncrementInt (Variables|Default|Gettimer))
                (:%20%20
                  (Variables|Default|Settimer _result_2)
                  (for (_array_element _array_index) (Variables|Default|Getschool)
                    (bind _astrawler (Utilities|Casting|CastToTrawler _array_element))
                    (Default|MovetoLocation _astrawler (Math|Integer|%(Integer) (+ _array_index (Variables|Default|GetcurrentPositionConfiguration)) 4)))))))
          (else
            ;;[1 1 1] Keep moving towards position
            (for (_array_element_2 _array_index_2) (Variables|Default|Getschool)
              (bind _astrawler_2 (Utilities|Casting|CastToTrawler _array_element_2))
              (Default|MovetoLocation _astrawler_2 (Math|Integer|%(Integer) (+ _array_index_2 (Variables|Default|GetcurrentPositionConfiguration)) (Utilities|Array|Length _school)))))))
      (:then_2
        ;;[1 1 1] Track every 10 seconds
        (Utilities|FlowControl|Delay 1.0)
        (bind _result_3 (Math|Integer|IncrementInt (Variables|Default|Gettimer))
          (:%20%20
            (bind _output_get (Variables|Default|Settimer _result_3))))))))

(fn GetTrawlerPositions
  (bind _asbarge (Utilities|Casting|CastToBarge (Components|GetOwner)))
  (bind _trawlerpositionsv2 (Default|GetTrawlerPositionV2 _asbarge))
  (return _trawlerpositionsv2))

(fn GetDetectOthers
  (bind _asbarge (Utilities|Casting|CastToBarge (Components|GetOwner)))
  (bind _detectothers (Default|GetDetectOthers _asbarge))
  (return _detectothers))